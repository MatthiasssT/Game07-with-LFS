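; BP_MetalLampCeiling is a procedural ceiling lamp fixture: a straight cable run with anchors at both ends and evenly spaced lamps along it.
; The construction script runs CreateCables, which repeats cable meshes along local X and adds a mirrored anchor at the far end.
; CreateLamps then centers downward-rotated lamp meshes on the run, with spacing adjusted by a multiplier.
; Each lamp gets a point light placed at its mesh's LightSocket.
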(event EventBeginPlay)

(event Collision|EventActorBeginOverlap
  (params (OtherActor :type Actor%20Object%20Reference)))

(event EventTick
  (params (DeltaSeconds :type Float%20%28single-precision%29)))

(fn ConstructionScript
  (Utilities|FlowControl|Sequence
    (:then_0
      (CallFunction|CreateCables))
    (:then_1
      (CallFunction|CreateLamps))))

(fn CreateCables
  (for _index (range 0 (- (Variables|Config|GetInstanceCount) 1))
    (LocalVariables|SetIndex _index)
    (Utilities|FlowControl|Sequence
      (:then_0
        (if (== (LocalVariables|GetIndex) 0)
          (bind _returnvalue (AddComponent|AddStaticMeshComponent false (Math|Transform|MakeTransform (Math|Vector|MakeVector (Variables|Config|GetAnchorOffset) 0.0 0.0))))
          (Components|StaticMesh|SetStaticMesh _returnvalue (Variables|Default|GetAnchorMesh))))
      (:then_1
        (bind _returnvalue_2 (AddComponent|AddStaticMeshComponent false (Math|Transform|MakeTransform (+ "0, 0, 0" (* "1.000000, 0, 0" (* (LocalVariables|GetIndex) (Variables|Default|GetInstanceLengh)))))))
        (Components|StaticMesh|SetStaticMesh _returnvalue_2 (Variables|Default|GetCableMesh)))
      (:then_2
        (if (== (LocalVariables|GetIndex) (- (Variables|Config|GetInstanceCount) 1))
          (bind _returnvalue_3 (AddComponent|AddStaticMeshComponent false (Math|Transform|MakeTransform (+ (+ "0, 0, 0" (* "1.000000, 0, 0" (* (LocalVariables|GetIndex) (Variables|Default|GetInstanceLengh)))) (* "1.000000, 0, 0" (Variables|Default|GetInstanceLengh)) (Math|Vector|MakeVector (* (Variables|Config|GetAnchorOffset) -1.0) 0.0 0.0)) (Math|Conversions|RotationFromXVector "-1.000000, 0, 0"))))
          (Components|StaticMesh|SetStaticMesh _returnvalue_3 (Variables|Default|GetAnchorMesh)))))))

(fn CreateLamps
  (if (> (Variables|Config|GetLampCount) 0)
    (LocalVariables|SetDistanceBetweenLamps (/ (/ (* (Variables|Config|GetInstanceCount) (Variables|Default|GetInstanceLengh)) (Math|Conversions|ToFloat(Integer) (Variables|Config|GetLampCount))) (Variables|Config|GetLampDistanceMultiplier)))
    (Utilities|FlowControl|Sequence
      (:then_0
        (LocalVariables|SetLampsHalfLength (/ (* (Variables|Config|GetLampCount) (LocalVariables|GetDistanceBetweenLamps)) 2.0))
        (LocalVariables|SetCableHalfLength (/ (* (Variables|Config|GetInstanceCount) (Variables|Default|GetInstanceLengh)) 2.0)))
      (:then_1
        (LocalVariables|SetAnchorPointLamps (- "0, 0, 0" (Math|Vector|MakeVector (LocalVariables|GetLampsHalfLength) 0.0 0.0)))
        (for _index (range 0 (- (Variables|Config|GetLampCount) 1))
          (LocalVariables|SetIndex _index)
          (Utilities|FlowControl|Sequence
            (:then_0
              (bind _returnvalue (AddComponent|AddStaticMeshComponent false (Math|Transform|MakeTransform (+ (+ (LocalVariables|GetAnchorPointLamps) (* "1.000000, 0, 0" (* (LocalVariables|GetIndex) (LocalVariables|GetDistanceBetweenLamps)))) (* "1.000000, 0, 0" (/ (LocalVariables|GetDistanceBetweenLamps) 2.0)) (Math|Vector|MakeVector (LocalVariables|GetCableHalfLength) 0.0 0.0)) (Math|Conversions|RotationFromXVector "0, 0,-1.000000"))))
              (Components|StaticMesh|SetStaticMesh _returnvalue (Variables|Default|GetLampMesh))
              (LocalVariables|SetNewLampComponent _returnvalue))
            (:then_1
              (AddComponent|AddPointLightComponent false (Math|Transform|MakeTransform (.location (Transformation|GetSocketTransform (LocalVariables|GetNewLampComponent) "LightSocket" "RTS_Actor")) (.rotation (Transformation|GetSocketTransform (LocalVariables|GetNewLampComponent) "LightSocket" "RTS_Actor")))))))))))