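; BP_StoneWindowLarge_A is a large stone window prop for the Historical Museum, with four window parts that can be posed open or closed.
; The construction script sets each part's relative roll from its own angle variable, clamped between 0 and 90 degrees.
; The third and fourth parts take their angles crosswise, from WindowAngle04 and WindowAngle03 respectively.
; The event graph holds only disabled placeholder events, so the Blueprint adds no runtime behavior.
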(event EventBeginPlay)

(event Collision|EventActorBeginOverlap
  (params (OtherActor :type Actor%20Object%20Reference)))

(event EventTick
  (params (DeltaSeconds :type Float%20%28single-precision%29)))

(fn ConstructionScript
  (Transformation|SetRelativeRotation (Variables|Default|GetSM_WindowPart_01) (Math|Rotator|MakeRotator (Math|Float|Clamp(Float) (Variables|Default|GetWindow%20Angle%2001) 0.0 9e+01) 0.0 0.0) false false)
  (Transformation|SetRelativeRotation (Variables|Default|GetSM_WindowPart_02) (Math|Rotator|MakeRotator (Math|Float|Clamp(Float) (Variables|Default|GetWindow%20Angle%2002) 0.0 9e+01) 0.0 0.0) false false)
  (Transformation|SetRelativeRotation (Variables|Default|GetSM_WindowPart_03) (Math|Rotator|MakeRotator (Math|Float|Clamp(Float) (Variables|Default|GetWindow%20Angle%2004) 0.0 9e+01) 0.0 0.0) false false)
  (Transformation|SetRelativeRotation (Variables|Default|GetSM_WindowPart_04) (Math|Rotator|MakeRotator (Math|Float|Clamp(Float) (Variables|Default|GetWindow%20Angle%2003) 0.0 9e+01) 0.0 0.0) false false))