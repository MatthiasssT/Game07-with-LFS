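; BP_DisplayCasePreset_02 is a museum display case preset that builds an optional railing arrangement from its RailingVariant setting.
; The construction script adds static mesh components at fixed relative transforms, alternating the Railing01 mesh with a 90-degree-yawed Railing02.
; Variants 1 to 4 are cumulative, each reusing the previous pieces through shared sequence branches and adding one more railing.
; The event graph holds only disabled placeholder events, so there is no runtime logic.
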(event EventBeginPlay)

(event Collision|EventActorBeginOverlap
  (params (OtherActor :type Actor%20Object%20Reference)))

(event EventTick
  (params (DeltaSeconds :type Float%20%28single-precision%29)))

(fn ConstructionScript
  (switch int (Variables|Default|GetRailing%20Variant)
    (:1
      (bind _returnvalue (AddComponent|AddStaticMeshComponent false (Math|Transform|MakeTransform "7.000000,-4.424534,79.951073") :!label _label))
      (Components|StaticMesh|SetStaticMesh _returnvalue (Variables|Default|GetRailing01)))
    (:2
      (Utilities|FlowControl|Sequence
        (:then_0
          (goto _label))
        (:then_1
          (bind _returnvalue_2 (AddComponent|AddStaticMeshComponent false (Math|Transform|MakeTransform "5.000000,-73.000000,79.951065" "0,90.000000, 0") :!label _label_2))
          (Components|StaticMesh|SetStaticMesh _returnvalue_2 (Variables|Default|GetRailing02)))))
    (:3
      (Utilities|FlowControl|Sequence
        (:then_0
          (goto _label))
        (:then_1
          (goto _label_2))
        (:then_2
          (bind _returnvalue_3 (AddComponent|AddStaticMeshComponent false (Math|Transform|MakeTransform "7.000000,-74.456612,79.951065") :!label _label_3))
          (Components|StaticMesh|SetStaticMesh _returnvalue_3 (Variables|Default|GetRailing01)))))
    (:4
      (Utilities|FlowControl|Sequence
        (:then_0
          (goto _label))
        (:then_1
          (goto _label_2))
        (:then_2
          (goto _label_3))
        (:then_3
          (bind _returnvalue_4 (AddComponent|AddStaticMeshComponent false (Math|Transform|MakeTransform "146.000000,-73.000000,79.951103" "0,90.000000, 0")))
          (Components|StaticMesh|SetStaticMesh _returnvalue_4 (Variables|Default|GetRailing02)))))))