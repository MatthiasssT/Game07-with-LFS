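; BP_DisplayCasePreset_01 is a museum display case preset with a configurable railing around it.
; The Construction Script switches on RailingVariant to spawn one to four Railing01 static mesh components at fixed relative transforms, forming successive sides of a square.
; Higher variants reuse the lower variants' spawn nodes through Sequences, so each adds one side to the previous layout.
; The event graph has no active logic.
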(event EventBeginPlay)

(event Collision|EventActorBeginOverlap
  (params (OtherActor :type Actor%20Object%20Reference)))

(event EventTick
  (params (DeltaSeconds :type Float%20%28single-precision%29)))

(fn ConstructionScript
  (switch int (Variables|Default|GetRailing%20Variant)
    (:1
      (bind _returnvalue (AddComponent|AddStaticMeshComponent false (Math|Transform|MakeTransform "6.596817,-4.731324,49.876720") :!label _label))
      (Components|StaticMesh|SetStaticMesh _returnvalue (Variables|Default|GetRailing01)))
    (:2
      (Utilities|FlowControl|Sequence
        (:then_0
          (goto _label))
        (:then_1
          (bind _returnvalue_2 (AddComponent|AddStaticMeshComponent false (Math|Transform|MakeTransform "3.215462,-6.209198,49.876728" "0,-90.000000, 0") :!label _label_2))
          (Components|StaticMesh|SetStaticMesh _returnvalue_2 (Variables|Default|GetRailing01)))))
    (:3
      (Utilities|FlowControl|Sequence
        (:then_0
          (goto _label))
        (:then_1
          (goto _label_2))
        (:then_2
          (bind _returnvalue_3 (AddComponent|AddStaticMeshComponent false (Math|Transform|MakeTransform "6.596817,-145.752075,49.876720") :!label _label_3))
          (Components|StaticMesh|SetStaticMesh _returnvalue_3 (Variables|Default|GetRailing01)))))
    (:4
      (Utilities|FlowControl|Sequence
        (:then_0
          (goto _label))
        (:then_1
          (goto _label_2))
        (:then_2
          (goto _label_3))
        (:then_3
          (bind _returnvalue_4 (AddComponent|AddStaticMeshComponent false (Math|Transform|MakeTransform "145.917877,-6.208755,49.876720" "0,-90.000000, 0")))
          (Components|StaticMesh|SetStaticMesh _returnvalue_4 (Variables|Default|GetRailing01)))))))