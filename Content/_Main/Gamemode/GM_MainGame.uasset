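; Main game mode that manages music and ambience and handles the player being caught.
; BeginPlay fades in music and looping rain and locks input to the game, and SwitchToChaseMusic swaps the music for the escape track.
; PlayerCaught shows the cursor and caught widget, then, only if escape music is valid, fades it out, plays a caught sound, silences the alarm and calls PlayerDead on the character.
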(event Custom|PlayerCaught
  (bind _returnvalue (Game|GetPlayerController 0))
  (Variables|/Script/Engine.PlayerController|SetbShowMouseCursor _returnvalue true)
  (Input|SetInputModeGameandUI _returnvalue 0 "DoNotLock" true false)
  (bind _returnvalue_2 (Game|ConstructObjectfromClass "/Game/_Main/UI/WBP_Caught.WBP_Caught_C"))
  (bind _output_get (Variables|Default|SetCaughtWidget _returnvalue_2))
  (UserInterface|Viewport|AddtoViewport _output_get 0)
  (Default|Fadein (Variables|Default|GetCaughtWidget))
  (bind _escapemuiscref (Variables|Default|GetEscapeMuiscRef)
    (:then
      (Audio|Components|Audio|FadeOut _escapemuiscref 0.3 0.0 "Linear" :!class /Script/Engine.AudioComponent)
      (Audio|PlaySound2D "/Game/_Main/AI/Audio/Caught.Caught" 1.0 1.0 0.0 0 0)
      (bind _returnvalue_3 (Actor|GetActorOfClass "/Game/_Main/Alarms/blueprints/BP_Alarm.BP_Alarm_C"))
      (Audio|Components|Audio|FadeOut (Variables|/Game/_Main/Alarms/blueprints/BP_Alarm.BP_Alarm_C|GetAlarmSound _returnvalue_3) 0.0 0.0 "Linear" :!class /Script/Engine.AudioComponent)
      (bind _asbp_main_character (Utilities|Casting|CastToBP_MainCharacter (Game|GetPlayerCharacter 0)))
      (Default|PlayerDead _asbp_main_character))
    (:else)))

(event Custom|SwitchToChaseMusic
  (Audio|Components|Audio|FadeOut (Variables|Default|GetMusicRef) 0.3 0.0 "Linear" :!class /Script/Engine.AudioComponent)
  (bind _returnvalue (Audio|SpawnSound2D "/Game/_Main/Music/Escaping.Escaping" 0.3 1.0 0.0 0))
  (Variables|Default|SetEscapeMuiscRef _returnvalue))

(event EventBeginPlay
  (bind _returnvalue (Game|GetPlayerController 0))
  (Utilities|FlowControl|Sequence
    (:then_0
      (bind _returnvalue_2 (Audio|SpawnSound2D "/Game/_Main/Music/Music.Music" 0.3 1.0 0.0 0))
      (bind _output_get (Variables|Default|SetMusicRef _returnvalue_2))
      (Audio|Components|Audio|FadeIn _output_get 0.4 1.0 0.0 "Linear" :!class /Script/Engine.AudioComponent))
    (:then_1
      (bind _returnvalue_3 (Audio|SpawnSound2D "/Game/_Main/Niagara/AudioFX/Rain_Loop.Rain_Loop" 0.2 1.0 0.0 0))
      (bind _output_get_2 (Variables|Default|SetRainRef _returnvalue_3))
      (Audio|Components|Audio|FadeIn _output_get_2 0.4 1.0 0.0 "Linear" :!class /Script/Engine.AudioComponent)
      (Variables|/Script/Engine.PlayerController|SetbShowMouseCursor _returnvalue false)
      (Input|SetInputModeGameOnly _returnvalue false))))

(fn ConstructionScript)