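; BP_Guard is an AI guard character that can catch the player or be taken down by them.
; An overlap radius toggles the takedown prompt; TakeDown plays the victim montage, flags guard and AI controller dead, ragdolls after a delay and returns alignment transform data.
; Catch plays a montage whose notify sphere-traces ahead and tells GM_MainGame once if the player is caught.
; Run raises walk speed, and modular body meshes follow the main mesh's pose.
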(event OnComponentBeginOverlap(TakeDownRadius)
  (params (OverlappedComponent :type Primitive%20Component%20Object%20Reference) (OtherActor :type Actor%20Object%20Reference) (OtherComp :type Primitive%20Component%20Object%20Reference) (OtherBodyIndex :type Integer) (bFromSweep :type Boolean) (SweepResult :type Hit%20Result%20Structure%20%28by%20ref%29))
  (if (and (Actor|ActorHasTag OtherActor "Player") (not (Variables|Default|GetIsDead?)))
    (Rendering|SetVisibility (Variables|Default|GetTakedownPromptWBP) true false)))

(event OnComponentEndOverlap(TakeDownRadius)
  (params (OverlappedComponent :type Primitive%20Component%20Object%20Reference) (OtherActor :type Actor%20Object%20Reference) (OtherComp :type Primitive%20Component%20Object%20Reference) (OtherBodyIndex :type Integer))
  (if (Actor|ActorHasTag OtherActor "Player")
    (Rendering|SetVisibility (Variables|Default|GetTakedownPromptWBP) false false)))

(event Custom|TakedownRagdoll
  (Utilities|FlowControl|Delay 1.27)
  (Physics|SetSimulatePhysics (Variables|Character|GetMesh) true)
  (Pawn|Components|CharacterMovement|SetMovementMode (Variables|Character|GetCharacterMovement) "MOVE_None" 0))

(event EventBeginPlay)

(event Collision|EventActorBeginOverlap
  (params (OtherActor :type Actor%20Object%20Reference)))

(event EventTick
  (params (DeltaSeconds :type Float%20%28single-precision%29)))

(event EventRun
  (Variables|/Script/Engine.CharacterMovementComponent|SetMaxWalkSpeed (Variables|Character|GetCharacterMovement) 5e+02))

(event EventCatch
  (bind _returnvalue (Transformation|GetActorLocation))
  (if (not (Variables|Default|GetIsAttackin?))
    (Animation|Montage|PlayMontage (Variables|Character|GetMesh) "/Game/_Main/AI/Animations/Caught/Catch_Montage.Catch_Montage"
      (:then
        (Variables|Default|SetIsAttackin? true))
      (:OnCompleted
        (Variables|Default|SetIsAttackin? false))
      (:OnNotifyBegin
        (bind (_outhit _returnvalue_2) (Collision|SphereTraceForObjects _returnvalue (+ (* (Transformation|GetActorForwardVector) 1.5e+02) _returnvalue) 0.0 (Utilities|Array|MakeArray "ObjectTypeQuery3") false 0 "None"))
        (if _returnvalue_2
          (if (Actor|ActorHasTag (.HitActor (Collision|BreakHitResult _outhit)) "Player")
            (Utilities|FlowControl|DoOnce false
              (:Completed
                (bind _asgm_main_game (Utilities|Casting|CastToGM_MainGame (Game|GetGameMode)))
                (Default|PlayerCaught _asgm_main_game)))))))))

(fn ConstructionScript
  (Components|SkinnedMesh|SetLeaderPoseComponent (Variables|Default|GetTorso) (Variables|Character|GetMesh) false false))

(fn TakeDown
  (if (Variables|Default|GetCanTakedown?)
    (Animation|PlayAnimMontage "/Game/_Main/Player/Animations/Takedown/Takedown_Victim_Montage.Takedown_Victim_Montage" 1.0 "None")
    (CallFunction|TakedownRagdoll)
    (Rendering|SetVisibility (Variables|Default|GetTakedownPromptWBP) false false)
    (Variables|Default|SetIsDead? true)
    (bind _asbp_ai_guard (Utilities|Casting|CastToBP_AI_Guard (AI|GetAIController self)))
    (Variables|/Game/_Main/AI/BP_AI_Guard.BP_AI_Guard_C|SetIsDead? _asbp_ai_guard true)
    (return (Transformation|GetWorldLocation (Variables|Default|GetRefMesh)) (Transformation|GetActorRotation) (Variables|Default|GetCanTakedown?) 0)))