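; Guard AI controller that runs the BT_Guard behavior tree and reacts to seeing the player.
; While the guard is not dead, successful sight perception of a Player-tagged actor sets the SeenPlayer blackboard key, which is never cleared here.
; The first sighting also plays a shout, then starts the level's BP_Alarm after a short delay.
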(event OnTargetPerceptionUpdated(AIPerception)
  (params (Actor :type Actor%20Object%20Reference) (Stimulus :type AI%20Stimulus%20Structure))
  (if (not (Variables|Default|GetIsDead?))
    (bind _returnvalue (Class|AIPerceptionSystem|GetSenseClassforStimulus Stimulus))
    (if (== _returnvalue "/Script/AIModule.AISense_Sight")
      (if (and (.bSuccessfullySensed (Utilities|Struct|BreakAIStimulus Stimulus)) (Actor|ActorHasTag Actor "Player"))
        (AI|Components|Blackboard|SetValueasBool (AI|GetBlackboard 0) (Utilities|Name|MakeLiteralName "SeenPlayer") true)
        (if (not (Variables|Default|GetHasSeenPlayer?))
          (Variables|Default|SetHasSeenPlayer? true)
          (Audio|PlaySoundatLocation "/Game/_Main/AI/Audio/MS_Shout.MS_Shout" (Transformation|GetActorLocation (Components|GetOwner (Variables|Default|GetAIPerception))) "0, 0, 0" 1.0 1.0 0.0 "/Game/_Main/Alarms/Sounds/SA_Sensor.SA_Sensor" 0 0 0)
          (Utilities|FlowControl|Delay 0.5)
          (bind _returnvalue_2 (Actor|GetActorOfClass "/Game/_Main/Alarms/blueprints/BP_Alarm.BP_Alarm_C"))
          (Default|StartAlarm _returnvalue_2))))))

(event EventBeginPlay
  (AI|RunBehaviorTree "/Game/_Main/AI/BT_Guard.BT_Guard"))

(fn ConstructionScript)