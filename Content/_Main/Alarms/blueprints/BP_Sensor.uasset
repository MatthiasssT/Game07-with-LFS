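; BP_Sensor is a detection device that raises the alarm when it detects an actor tagged Player.
; Its DetectPlayer event fires only once, guarded by a HasDetected flag that is never reset here.
; On detection it plays a camera shutter sound, starts the alarm on the BP_Alarm found by class lookup, and drives the point light's intensity through a timeline, like a camera flash.
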(event Custom|DetectPlayer
  (params (ActorDetected :type Actor%20Object%20Reference))
  (if (and (Actor|ActorHasTag ActorDetected "Player") (not (Variables|Default|GetHasDetected?)))
    (Variables|Default|SetHasDetected? true)
    (Audio|PlaySoundatLocation "/Engine/VREditor/Sounds/UI/Camera_Shutter.Camera_Shutter" (Transformation|GetActorLocation) "0, 0, 0" 1.0 1.0 0.0 "/Game/_Main/Alarms/Sounds/SA_Sensor.SA_Sensor" 0 0 0)
    (bind _returnvalue (Actor|GetActorOfClass "/Game/_Main/Alarms/blueprints/BP_Alarm.BP_Alarm_C"))
    (Default|StartAlarm _returnvalue)
    (bind _intensity (Timeline|PointLightTimeline Play)
      (:Update
        (Rendering|Components|Light|SetIntensity (Variables|Default|GetPointLight) (Math|Float|Lerp 0.0 5e+04 _intensity))))))

(fn ConstructionScript)