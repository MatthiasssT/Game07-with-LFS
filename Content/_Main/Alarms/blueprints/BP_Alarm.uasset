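; Alarm actor that sounds an alarm and puts the level's guards into pursuit of the player.
; StartAlarm plays the alarm sound at its location once, guarded by IsAlarmActive, then calls AlertGuards.
; AlertGuards sets the SeenPlayer blackboard key on every BP_Guard's AI controller and switches GM_MainGame to chase music.
; StopAlarm fades out the sound but leaves IsAlarmActive set, so the alarm cannot restart.
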(event Custom|Start%20Alarm
  (if (not (Variables|Default|GetIsAlarmActive))
    (bind _returnvalue (Audio|SpawnSoundatLocation "/Game/_Main/Alarms/Sounds/MS_Alarm.MS_Alarm" (Transformation|GetActorLocation) "0, 0, 0" 1.0 1.0 0.0 0 0))
    (Variables|Default|SetAlarmSound _returnvalue)
    (Variables|Default|SetIsAlarmActive true)
    (CallFunction|AlertGuards)))

(event Custom|Stop%20Alarm
  (if (Variables|Default|GetIsAlarmActive)
    (Audio|Components|Audio|FadeOut (Variables|Default|GetAlarmSound) 1.0 0.0 "Linear" :!class /Script/Engine.AudioComponent)))

(event Custom|AlertGuards
  (bind _outactors (Actor|GetAllActorsOfClass "/Game/_Main/AI/BP_Guard.BP_Guard_C"))
  (for _array_element _outactors
    (bind _asbp_ai_guard (Utilities|Casting|CastToBP_AI_Guard (AI|GetAIController _array_element)))
    (AI|Components|Blackboard|SetValueasBool (AI|GetBlackboard _asbp_ai_guard) (Utilities|Name|MakeLiteralName "SeenPlayer") true))
  (bind _asgm_main_game (Utilities|Casting|CastToGM_MainGame (Game|GetGameMode)))
  (Default|SwitchtoChaseMusic _asgm_main_game))

(fn ConstructionScript)