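; BP_Lever is an interactable lever that triggers an assigned output actor and animates between two positions.
; Interacting calls SwitchLever, which plays a sound, then sends InteractMessage to OutputActor if it is valid and implements BPI_Interact.
; Only then does it toggle IsActivated and play or reverse the LeverPulled timeline, which interpolates the lever's relative rotation.
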(event Custom|SwitchLever
  (Audio|PlaySoundatLocation "/Engine/VREditor/Sounds/UI/Floating_UI_Close.Floating_UI_Close" (Transformation|GetActorLocation) "0, 0, 0" 1.0 1.0 0.0 "/Game/_Main/Alarms/Sounds/SA_Sensor.SA_Sensor" 0 0 0)
  (bind _outputactor (Variables|Default|GetOutputActor)
    (:then
      (if (Utilities|DoesObjectImplementInterface _outputactor "/Game/_Main/Interface/BPI_Interact.BPI_Interact_C")
        (Class|BPIInteract|Interact(Message) _outputactor)
        (if (not (Variables|Default|GetIsActivated?))
          (Variables|Default|SetIsActivated? true)
          (bind _rotatelever (Timeline|leverPulled Play)
            (:Update
              (Transformation|SetRelativeRotation (Variables|Default|GetLever) (Math|Rotator|Lerp(Rotator) "135.000000,0.000000,0.000000" "45.000000,0.000000,0.000000" _rotatelever) false false)))
          (else
            (Variables|Default|SetIsActivated? false)
            (Timeline|leverPulled Reverse)))))
    (:else)))

(event EventInteract
  (CallFunction|SwitchLever))

(fn ConstructionScript)