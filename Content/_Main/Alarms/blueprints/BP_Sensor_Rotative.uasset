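; Rotating alarm sensor that detects the player who lingers inside its detection mesh.
; A timeline, alternately played and reversed through a FlipFlop, sweeps the head back and forth.
; Overlap by a Player-tagged actor starts a looping timer that fills the UI detection bar, then calls DetectPlayer and shows detection text at the threshold.
; Leaving the mesh stops the timer and resets progress, clearing the bar unless already detected.
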(event OnComponentBeginOverlap(TriggerDetectionMesh)
  (params (OverlappedComponent :type Primitive%20Component%20Object%20Reference) (OtherActor :type Actor%20Object%20Reference) (OtherComp :type Primitive%20Component%20Object%20Reference) (OtherBodyIndex :type Integer) (bFromSweep :type Boolean) (SweepResult :type Hit%20Result%20Structure%20%28by%20ref%29))
  (if (Actor|ActorHasTag OtherActor "Player")
    (Variables|Default|SetPlayerInZone? true)
    (bind _returnvalue (Utilities|Time|SetTimerbyEvent (delegate Custom|Count) 0.002 true))
    (Variables|Default|SetCountTimer _returnvalue)))

(event OnComponentEndOverlap(TriggerDetectionMesh)
  (params (OverlappedComponent :type Primitive%20Component%20Object%20Reference) (OtherActor :type Actor%20Object%20Reference) (OtherComp :type Primitive%20Component%20Object%20Reference) (OtherBodyIndex :type Integer))
  (bind _playerref (Variables|Default|GetPlayerRef))
  (bind _gameuiref (Variables|/Game/_Main/Player/BP_MainCharacter.BP_MainCharacter_C|GetGameUiRef _playerref))
  (if (Actor|ActorHasTag OtherActor "Player")
    (Variables|Default|SetPlayerInZone? false)
    (Utilities|Time|ClearandInvalidateTimerbyHandle (Variables|Default|GetCountTimer))
    (Variables|Default|SetTimeInZone 0.0)
    (if (not (Variables|/Game/_Main/UI/WBP_GameUI.WBP_GameUI_C|GetDetected? _gameuiref))
      (Progress|SetPercent (Variables|/Game/_Main/UI/WBP_GameUI.WBP_GameUI_C|GetDetectionBar _gameuiref) 0.0))))

(event Custom|Count
  (Variables|Default|SetTimeInZone (+ (Variables|Default|GetTimeInZone) 0.005))
  (CallFunction|UpdateProgressBar)
  (if (>= (Variables|Default|GetTimeInZone) 3.0)
    (CallFunction|DetectPlayer (stale OnComponentBeginOverlap(TriggerDetectionMesh) OtherActor))
    (Utilities|Time|ClearandInvalidateTimerbyHandle (Variables|Default|GetCountTimer))
    (Default|DetectionText (Variables|/Game/_Main/Player/BP_MainCharacter.BP_MainCharacter_C|GetGameUiRef (Variables|Default|GetPlayerRef)))))

(event Custom|Update%20Progress%20Bar
  (bind _playerref (Variables|Default|GetPlayerRef))
  (bind _gameuiref (Variables|/Game/_Main/Player/BP_MainCharacter.BP_MainCharacter_C|GetGameUiRef _playerref))
  (if (not (Variables|/Game/_Main/UI/WBP_GameUI.WBP_GameUI_C|GetDetected? _gameuiref))
    (Progress|SetPercent (Variables|/Game/_Main/UI/WBP_GameUI.WBP_GameUI_C|GetDetectionBar _gameuiref) (/ (Variables|Default|GetTimeInZone) 3.0))))

(event EventBeginPlay
  (Utilities|FlowControl|Sequence
    (:then_0
      (bind _rotation (Timeline|MotionTimeline Play)
        (:Update
          (Transformation|SetRelativeRotation (Variables|Default|GetHead) (Math|Rotator|Lerp(Rotator) "0.000000,180.000000,0.000000" "0, 0, 0" _rotation) false false))
        (:Finished
          (Utilities|FlowControl|FlipFlop
            (:A
              (Timeline|MotionTimeline Reverse))
            (:B
              (Timeline|MotionTimeline Play))))))
    (:then_1
      (bind _asbp_main_character (Utilities|Casting|CastToBP_MainCharacter (Game|GetPlayerCharacter 0)))
      (Variables|Default|SetPlayerRef _asbp_main_character))))

(fn ConstructionScript
  (|CallParentFunction))